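; Wire puzzle actor where the player clicks five cables loose in the order set by the SequenceWin string.
; The construction script builds material-coded cables between endpoint components, each mapped to a collision box.
; Interaction switches to the puzzle view with mouse cursor and binds the character's SendPuzzleWire dispatcher, which reports clicked boxes.
; Correct clicks detach cables until the win restores character control; a wrong click reattaches all and exits, as does E.
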(event `self.ReceiveBeginPlay`
  (bind _keys (`BlueprintMapLibrary.Map_Keys` (`self.Cables`)))
  (for (_array_element _array_index) _keys
    (`CableComponent.SetAttachEndToComponent` _array_element (`|GetArrayItem` (`self.EndPoints`) _array_index) "None")
    (set `self.Win` false)))

(event `/Game/BPI_Interact.Interaction`
  (params (DirectionInteract :type "Vector Structure") (PlayerRef :type "/Game/ThirdPerson/Blueprints/BP_ThirdPersonCharacter Object Reference"))
  (bind _returnvalue (`GameplayStatics.GetPlayerController` 0))
  (set `/Game/ThirdPerson/Blueprints/BP_ThirdPersonCharacter.WirePuzzleMode` true PlayerRef)
  (`PlayerController.SetViewTargetWithBlend` (`GameplayStatics.GetPlayerController` 0) self 0.0 "VTBlend_Linear" 0.0 false)
  (`WidgetBlueprintLibrary.SetInputMode_GameAndUIEx` _returnvalue null)
  (set `PlayerController.bShowMouseCursor` true _returnvalue)
  (add `/Game/ThirdPerson/Blueprints/BP_ThirdPersonCharacter.SendPuzzleWire` PlayerRef (`|CreateDelegate` :!event `SendPuzzleWire_Event`))
  (`self.EnableInput` (`GameplayStatics.GetPlayerController` 0)))

(event `SendPuzzleWire_Event`
  (params (WireCollision :type "BoxComponent Object Reference"))
  (bind _returnvalue (`GameplayStatics.GetPlayerController` 0))
  (bind _values (`BlueprintMapLibrary.Map_Values` (`self.Cables`)))
  (bind _output_get (set `self.ClickedCableNum` (`KismetArrayLibrary.Array_Find` _values WireCollision)))
  (if (>= _output_get 0)
    (if (== (+ (`self.ClickedCableNum`) 1) (`KismetStringLibrary.Conv_StringToInt` (`|GetArrayItem` (`KismetStringLibrary.GetCharacterArrayFromString` (`self.SequenceWin`)) (`self.CurrentCable`))))
      (bind _keys (`BlueprintMapLibrary.Map_Keys` (`self.Cables`)))
      (set `CableComponent.bAttachEnd` false (`|GetArrayItem` _keys (`self.ClickedCableNum`)))
      (bind _result (`/Engine/EditorBlueprintResources/StandardMacros.IncrementInt` (`self.CurrentCable`))
        (:`  `
          (if (>= _result 5)
            (`KismetSystemLibrary.PrintString` "WIN")
            (set `self.Win` true)
            (`GameplayStatics.PlaySound2D` "/Game/Music/son_Lost_record/zap_2_sec.zap_2_sec" 1.0 1.0 0.0 null null)
            (`Controller.Possess` _returnvalue (cast `/Game/ThirdPerson/Blueprints/BP_ThirdPersonCharacter` (`GameplayStatics.GetPlayerCharacter` 0) :!pure true))
            (`WidgetBlueprintLibrary.SetInputMode_GameOnly` _returnvalue)
            (set `PlayerController.bShowMouseCursor` false _returnvalue)
            (else
              (`GameplayStatics.PlaySound2D` "/Game/Music/son_Lost_record/zap_2_sec.zap_2_sec" 1.0 1.0 0.0 null null)))))
      (else
        (`KismetSystemLibrary.PrintString` "FALSE")
        (set `self.Win` false)
        (bind _keys_2 (`BlueprintMapLibrary.Map_Keys` (`self.Cables`)))
        (for _array_element _keys_2
          (set `CableComponent.bAttachEnd` true _array_element))
        (set `self.CurrentCable` 0)
        (set `self.ClickedCableNum` 0)
        (`self.Reset`)))))

(event `Reset`
  (bind _returnvalue (`GameplayStatics.GetPlayerController` 0))
  (bind _asbp_third_person_character (cast `/Game/ThirdPerson/Blueprints/BP_ThirdPersonCharacter` (`GameplayStatics.GetPlayerCharacter` 0) :!label _label))
  (set `/Game/ThirdPerson/Blueprints/BP_ThirdPersonCharacter.WirePuzzleMode` false _asbp_third_person_character)
  (`PlayerController.SetViewTargetWithBlend` (`GameplayStatics.GetPlayerController` 0) _asbp_third_person_character 0.0 "VTBlend_Linear" 0.0 false)
  (`self.DisableInput` _returnvalue)
  (`self.EnableInput` _asbp_third_person_character _returnvalue)
  (set `PlayerController.bShowMouseCursor` false _returnvalue)
  (`WidgetBlueprintLibrary.SetInputMode_GameOnly` _returnvalue))

(event `Key|E`
  (params (Key :type "Key Structure"))
  (:`Pressed`
    (goto _label)))

(fn `UserConstructionScript`
  (locals (StartingPoints :type "Array of SceneComponent Object Reference"))
  (`BlueprintMapLibrary.Map_Clear` (`self.Cables`))
  (set `local.StartingPoints` (`|MakeArray` (`self.Cable1Start`) (`self.Cable2Start`) (`self.Cable3Start`) (`self.Cable4Start`) (`self.Cable5Start`)))
  (set `self.EndPoints` (`|MakeArray` (`self.Cable1End`) (`self.Cable2End`) (`self.Cable3End`) (`self.Cable4End`) (`self.Cable5End`)))
  (for (_array_element _array_index) (`local.StartingPoints`)
    (bind _returnvalue (`AddComponent|NODE_AddCableComponent-0`))
    (bind (_relativelocation_x _relativelocation_y _relativelocation_z) (`KismetMathLibrary.BreakVector` (`SceneComponent.RelativeLocation` _array_element)))
    (bind _returnvalue_2 (`AddComponent|NODE_AddBoxComponent-0` :`RelativeTransform` (`KismetMathLibrary.MakeTransform` (`KismetMathLibrary.MakeVector` 0.0 _relativelocation_y _relativelocation_z) (struct) (1.0 1.0 2.0))))
    (`SceneComponent.K2_AttachToComponent` _returnvalue _array_element "None" "KeepRelative" "KeepRelative" "KeepRelative" true)
    (`CableComponent.SetAttachEndToComponent` _returnvalue (`|GetArrayItem` (`self.EndPoints`) _array_index) "None")
    (`BlueprintMapLibrary.Map_Add` (`self.Cables`) _returnvalue _returnvalue_2)
    (`PrimitiveComponent.SetMaterial` _returnvalue 0 (`|GetArrayItem` (`self.Material`) _array_index))))