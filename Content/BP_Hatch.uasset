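; BP_Hatch is a roof hatch that opens with a key and has a trigger that ends the game with a win screen.
; Its Interaction event checks only the player's first inventory item for "Key", then runs a one-time timeline that rotates RoofHatch open.
; Separately, the Box overlap shows Win_Menu for BP_ThirdPersonCharacter with UI-only input and a cursor, without checking whether the hatch is open.
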(event `/Game/BPI_Interact.Interaction`
  (params (DirectionInteract :type "Vector Structure") (PlayerRef :type "/Game/ThirdPerson/Blueprints/BP_ThirdPersonCharacter Object Reference"))
  (if (== (`.Item_Name_2_634492BF42674EF4DC449DA84C3E2BCD` (break `/Game/InventorySystem/ItemInformation` (`|GetArrayItem` (`/Game/ThirdPerson/Blueprints/BP_ThirdPersonCharacter.ItemsArray` PlayerRef)))) "Key")
    (`/Engine/EditorBlueprintResources/StandardMacros.DoOnce` false
      (:`Completed`
        (bind (_direction _rotation) (`Timeline|Timeline` :!via `PlayFromStart`)
          (:`Update`
            (`SceneComponent.K2_SetRelativeRotation` (`self.Roof_Hatch`) (`KismetMathLibrary.RLerp` (struct :`Roll` -270.0) (struct :`Roll` -180.0) _rotation) false false)))))))

(event `self.Box.OnComponentBeginOverlap`
  (params (OverlappedComponent :type "PrimitiveComponent Object Reference") (OtherActor :type "Actor Object Reference") (OtherComp :type "PrimitiveComponent Object Reference") (OtherBodyIndex :type Integer) (bFromSweep :type Boolean) (SweepResult :type "HitResult Structure (by ref)"))
  (bind _returnvalue (`GameplayStatics.GetPlayerController` 0))
  (cast `/Game/ThirdPerson/Blueprints/BP_ThirdPersonCharacter` OtherActor)
  (bind _returnvalue_2 (`|CreateWidget` "/Game/UI/BP/Win_Menu.Win_Menu_C"))
  (`UserWidget.AddToViewport` _returnvalue_2 0)
  (`WidgetBlueprintLibrary.SetInputMode_UIOnlyEx` _returnvalue _returnvalue_2)
  (set `PlayerController.bShowMouseCursor` true _returnvalue))

(fn `UserConstructionScript`)