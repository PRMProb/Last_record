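; BP_AddQTE is a trigger actor that starts music and randomly timed quick-time events for the player.
; When BP_ThirdPersonCharacter overlaps its box, it adds the character's QTE widget, plays a 2D track and starts a looping timer.
; Each timer tick has a small random chance, if no QTE is launched, to set the character's QTELaunched flag and play the widget's QTE after a short delay.
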(event `self.ReceiveBeginPlay`)

(event `self.Box.OnComponentBeginOverlap`
  (params (OverlappedComponent :type "PrimitiveComponent Object Reference") (OtherActor :type "Actor Object Reference") (OtherComp :type "PrimitiveComponent Object Reference") (OtherBodyIndex :type Integer) (bFromSweep :type Boolean) (SweepResult :type "HitResult Structure (by ref)"))
  (bind _asbp_third_person_character (cast `/Game/ThirdPerson/Blueprints/BP_ThirdPersonCharacter` OtherActor))
  (bind _output_get (set `self.RefPlayer` _asbp_third_person_character))
  (`/Game/ThirdPerson/Blueprints/BP_ThirdPersonCharacter.AddQTEWidget` _output_get)
  (`GameplayStatics.PlaySound2D` "/Game/QTEMusic/Coding_and_Canvas_Dreams.Coding_and_Canvas_Dreams" 1.0 1.0 0.0 null null)
  (`KismetSystemLibrary.K2_SetTimerDelegate` (delegate `CustomEvent`) 0.75 true))

(event `CustomEvent`
  (bind _refplayer (`self.RefPlayer`))
  (if (not (`/Game/ThirdPerson/Blueprints/BP_ThirdPersonCharacter.QTELaunched` _refplayer))
    (if (<= (`KismetMathLibrary.RandomFloat`) 0.2)
      (set `/Game/ThirdPerson/Blueprints/BP_ThirdPersonCharacter.QTELaunched` true _refplayer)
      (`KismetSystemLibrary.Delay` 1.0)
      (`/Game/QTEMusic/WG_QTE.PlayQTE` (`.QTERef` (`/Game/ThirdPerson/Blueprints/BP_ThirdPersonCharacter.QTERef` (`self.RefPlayer`)))))))

(fn `UserConstructionScript`)