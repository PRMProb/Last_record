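; BP_MasterItem is a pickup actor for the inventory system, likely serving as the base for item Blueprints.
; Its collision component enables input when a BP_ThirdPersonCharacter overlaps, caching that character, and disables input on any end overlap.
; While input is enabled, pressing E passes ItemDetails to the character's PickItemsInSlot, then destroys the item without checking a result.
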(event `Key|E`
  (params (Key :type "Key Structure"))
  ;[0.05098 0.05098 0.05098] Pick Items
  (:`Pressed`
    (`/Game/ThirdPerson/Blueprints/BP_ThirdPersonCharacter.PickItemsInSlot` (`self.CharacterCast`) (`self.ItemDetails`))
    (`self.K2_DestroyActor`)))

(event `self.Collision.OnComponentBeginOverlap`
  (params (OverlappedComponent :type "PrimitiveComponent Object Reference") (OtherActor :type "Actor Object Reference") (OtherComp :type "PrimitiveComponent Object Reference") (OtherBodyIndex :type Integer) (bFromSweep :type Boolean) (SweepResult :type "HitResult Structure (by ref)"))
  ;[0.05098 0.05098 0.05098] Enable Input ONLY inside Collison
  (bind _asbp_third_person_character (cast `/Game/ThirdPerson/Blueprints/BP_ThirdPersonCharacter` OtherActor))
  (set `self.CharacterCast` _asbp_third_person_character)
  (`self.EnableInput` (`GameplayStatics.GetPlayerController` 0)))

(event `self.Collision.OnComponentEndOverlap`
  (params (OverlappedComponent :type "PrimitiveComponent Object Reference") (OtherActor :type "Actor Object Reference") (OtherComp :type "PrimitiveComponent Object Reference") (OtherBodyIndex :type Integer))
  ;[0.05098 0.05098 0.05098] Enable Input ONLY inside Collison
  (`self.DisableInput` (`GameplayStatics.GetPlayerController` 0)))

(fn `UserConstructionScript`)